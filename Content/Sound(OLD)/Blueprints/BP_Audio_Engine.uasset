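; Engine audio Blueprint that drives a sports car engine MetaSound for the player's car.
; On BeginPlay it starts the sound and binds to SportsCar_Pawn events, forwarding throttle and gear changes as triggers, camera switches as a perspective parameter, and restarting on reset.
; Tick feeds normalized RPM, forward speed and absolute throttle into the MetaSound.
; It also times positive throttle input, so releasing after a sustained press fires a blowoff.
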(event `self.ReceiveTick`
  (params (DeltaSeconds :type "Float (single-precision)"))
  (`self.UpdateMetasoundValues`)
  (`self.CountThrottleTime`))

(event `self.ReceiveBeginPlay`
  ;[1 1 1] Play Engine Metasound
  (`AudioComponent.Play` (`self.MS_Engine_SportsCar`) 0.0)
  ;[1 1 1] Get Sports Car Actor
  (bind _assports_car_pawn (cast `/Game/VehicleTemplate/Blueprints/SportsCar/SportsCar_Pawn` (`GameplayStatics.GetPlayerPawn` 0)))
  (set `self.CarParent` _assports_car_pawn)
  ;[1 1 1] Bind ThrottleOn Event
  (add `/Game/VehicleTemplate/Blueprints/SportsCar/SportsCar_Pawn.ThrottleOnEvent` (`self.CarParent`) (delegate `ThrottleOnEvent_Event_0`))
  ;[1 1 1] Bind ThrottleOff Event
  (add `/Game/VehicleTemplate/Blueprints/SportsCar/SportsCar_Pawn.ThrottleOffEvent` (`self.CarParent`) (delegate `ThrottleOffEvent_Event`))
  ;[1 1 1] Bind GearChange Event
  (add `/Game/VehicleTemplate/Blueprints/SportsCar/SportsCar_Pawn.GearChangeEvent` (`self.CarParent`) (delegate `GearChangeEvent_Event`))
  ;[1 1 1] Bind ResetCar Event
  (add `/Game/VehicleTemplate/Blueprints/SportsCar/SportsCar_Pawn.ResetCar` (`self.CarParent`) (delegate `ResetCar_Event`))
  ;[1 1 1] Bind camera switch
  (add `/Game/VehicleTemplate/Blueprints/SportsCar/SportsCar_Pawn.SwitchCamera` (`self.CarParent`) (delegate `SwitchCamera_Event`)))

(event `ThrottleOffEvent_Event`
  ;[1 1 1] Bind ThrottleOff Event
  (`AudioParameterControllerInterface.SetTriggerParameter` (`self.MS_Engine_SportsCar`) "ThrottleOff")
  (if (> (`self.ThrottleTime`) 1.5)
    (`AudioParameterControllerInterface.SetTriggerParameter` (`self.MS_Engine_SportsCar`) "Blowoff")))

(event `ThrottleOnEvent_Event_0`
  ;[1 1 1] Bind ThrottleOn Event
  (`AudioParameterControllerInterface.SetTriggerParameter` (`self.MS_Engine_SportsCar`) "ThrottleOn"))

(event `ResetCar_Event`
  (bind _ms_engine_sportscar (`self.MS_Engine_SportsCar`))
  ;[1 1 1] Bind ResetCar Event
  (`AudioComponent.Stop` _ms_engine_sportscar)
  (`KismetSystemLibrary.Delay` 0.2)
  (`AudioComponent.Play` _ms_engine_sportscar 0.0))

(event `SwitchCamera_Event`
  (params (Camera :type "Float (double-precision)"))
  ;[1 1 1] Bind camera switch
  (`AudioParameterControllerInterface.SetFloatParameter` (`self.MS_Engine_SportsCar`) "Perspective" Camera))

(event `GearChangeEvent_Event`
  ;[1 1 1] Bind GearChange Event
  (`AudioParameterControllerInterface.SetTriggerParameter` (`self.MS_Engine_SportsCar`) "GearChange"))

(fn `CountThrottleTime`
  ;[1 1 1] Check if player is on throttle of off throttle
  (if (> (`self.ThrottleInput`) 0.0)
    ;[1 1 1] If throttle is on, increment timer variable
    (set `self.ThrottleTime` (+ (`GameplayStatics.GetWorldDeltaSeconds`) (`self.ThrottleTime`)))
    (else
      ;[1 1 1] If throttle is off, reset timer
      (set `self.ThrottleTime` 0.0))))

(fn `UpdateMetasoundValues`
  ;[1 1 1] Normalize RPM
  (`AudioParameterControllerInterface.SetFloatParameter` (`self.MS_Engine_SportsCar`) "NormalizedRPM" (`KismetMathLibrary.NormalizeToRange` (`self.RPMCurrent`) 0.0 (`self.RPMMax`)))
  ;[1 1 1] Forward Speed
  (`AudioParameterControllerInterface.SetFloatParameter` (`self.MS_Engine_SportsCar`) "NormalizedSpeedForward" (`KismetMathLibrary.NormalizeToRange` (`self.ForwardSpeed`) 0.0 5500.0))
  ;[1 1 1] Throttle
  (`AudioParameterControllerInterface.SetFloatParameter` (`self.MS_Engine_SportsCar`) "Throttle" (`KismetMathLibrary.Abs` (`self.ThrottleInput`))))

(fn `UserConstructionScript`)