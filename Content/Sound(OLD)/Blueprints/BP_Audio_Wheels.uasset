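; Wheel audio Blueprint for the player's sports car, driving a MetaSound wheel loop and track bumper hits.
; Each tick feeds skid, rotation velocity and ground contact into the wheel sound.
; While moving, a downward trace resolves the surface through SurfaceSoundData and swaps the MetaSound, or plays a one-shot speed/throttle-driven bumper on bumper surfaces.
; SuspensionTrigger, uncalled here, also plays the bumper near full normalized suspension length.
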(event `self.ReceiveBeginPlay`
  (`AudioComponent.Play` (`self.MS_WheelTemplate`) 0.0)
  ;[1 1 1] Get Sports Car Actor
  (bind _assports_car_pawn (cast `/Game/VehicleTemplate/Blueprints/SportsCar/SportsCar_Pawn` (`GameplayStatics.GetPlayerPawn` 0)))
  (set `self.CarParent` _assports_car_pawn))

(event `self.ReceiveTick`
  (params (DeltaSeconds :type "Float (single-precision)"))
  (`self.UpdateSkidAndVelocity`)
  (`self.Update Wheel Surface`))

(fn `SuspensionTrigger`
  (locals (CanTriggerSuspensionSound :type Boolean))
  (bind _normalizedsuspensionlength (`self.NormalizedSuspensionLength`))
  (`KismetSystemLibrary.PrintString` (`KismetStringLibrary.Conv_DoubleToString` _normalizedsuspensionlength))
  (`/Engine/EditorBlueprintResources/StandardMacros.CompareFloat` _normalizedsuspensionlength 0.99
    (:`>`
      (`AudioComponent.Play` (`self.TrackBumper`) 0.0 :!label _label)
      (set `local.CanTriggerSuspensionSound` false))
    (:`==`
      (goto _label))
    (:`<`
      (`/Engine/EditorBlueprintResources/StandardMacros.CompareFloat` (`self.NormalizedSuspensionLength`) 0.9
        (:`<`
          (`/Engine/EditorBlueprintResources/StandardMacros.DoOnce` false
            (:`Completed`
              (set `local.CanTriggerSuspensionSound` true))))))))

(fn `Update Wheel Surface`
  (locals (CurrentWheelSurface :type "MetaSoundSource Object Reference") (NewWheelSurface :type "MetaSoundSource Object Reference") (BumperSurface :type "MetaSoundSource Object Reference" :default null) (CanPlayBumper :type Boolean :default true))
  (bind _returnvalue (`self.K2_GetActorLocation`))
  (bind _trackbumper (`self.TrackBumper`))
  (bind _ms_wheeltemplate (`self.MS_WheelTemplate`))
  (bind _sound (`AudioComponent.Sound` (`self.MS_WheelTemplate`)))
  ;[1 1 1] Check If car is moving
  (`/Engine/EditorBlueprintResources/StandardMacros.CompareFloat` (`self.CarForwardSpeed`) 0.1
    (:`>`
      ;[1 1 1] Line Trace to get phys mat
      (bind (_outhit _returnvalue_2) (`KismetSystemLibrary.LineTraceSingle` _returnvalue (- _returnvalue (0.0 0.0 1000.0)) "TraceTypeQuery1" false (`|MakeArray` (`self.CarParent`) :!type "Actor Object Reference")))
      (if _returnvalue_2
        (bind _surfaceout (`/Game/Sound(OLD)/Data/SurfaceSoundData.ResolveSurfaceType` (`self.SurfaceSoundData`) _outhit))
        (set `local.NewWheelSurface` _surfaceout)
        ;[1 1 1] Check if material has changed
        (cast `MetaSoundSource` _sound)
        (if (!= (`KismetSystemLibrary.GetObjectName` (`local.NewWheelSurface`)) (`KismetSystemLibrary.GetObjectName` _sound))
          ;[1 1 1] Check surface to play bumper sound
          (if (!= (`KismetSystemLibrary.GetObjectName` (`local.NewWheelSurface`)) (`KismetSystemLibrary.GetObjectName` (`local.BumperSurface`)))
            ;[1 1 1] Stop old surface sound, start new surface sound
            (`AudioComponent.Stop` (`self.MS_WheelTemplate`))
            (`AudioComponent.SetSound` _ms_wheeltemplate (`local.NewWheelSurface`))
            (`AudioComponent.Play` _ms_wheeltemplate 0.0)
            (set `local.CanPlayBumper` true)
            (else
              ;[1 1 1] Bumper Sound
              (if (`local.CanPlayBumper`)
                (`AudioParameterControllerInterface.SetFloatParameter` _trackbumper "Speed" (`KismetMathLibrary.NormalizeToRange` (`self.CarForwardSpeed`) 0.0 5500.0))
                (`AudioParameterControllerInterface.SetFloatParameter` _trackbumper "Throttle" (`self.ThrottleInput`))
                (`AudioComponent.Play` _trackbumper 0.0)
                (set `local.CanPlayBumper` false)))))))))

(fn `UpdateSkidAndVelocity`
  (`AudioParameterControllerInterface.SetFloatParameter` (`self.MS_WheelTemplate`) "SkidMagnitude" (`KismetMathLibrary.Abs` (`KismetMathLibrary.NormalizeToRange` (`self.SkidMagnitude`) 0.0 2400.0)))
  (`AudioParameterControllerInterface.SetFloatParameter` (`self.MS_WheelTemplate`) "RotationVelocityNormalized" (`self.RotationVelocity`))
  (`AudioParameterControllerInterface.SetFloatParameter` (`self.MS_WheelTemplate`) "IsTouchingGround" (`KismetMathLibrary.Conv_BoolToDouble` (`self.IsTouchingGround`))))

(fn `UserConstructionScript`)